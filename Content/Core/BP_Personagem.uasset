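; Player character for a flap-to-fly bird, driven by the Jump input.
; Pressing Jump applies a scaled vertical impulse to the capsule and rotates the Bird component's roll by Sustain while it is within a positive range.
; Releasing Jump sets EstaCaindo (falling), which makes Tick add Decay to the roll every frame within set limits, without delta-time scaling.
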(event EventTick
  (params (DeltaSeconds :type Float%20%28single-precision%29))
  (bind _bird (Variables|Default|Getbird))
  (bind _returnvalue (Transformation|GetWorldRotation _bird))
  (Utilities|FlowControl|Sequence
    (:then_0
      (if (Variables|Default|GetEstaCaindo)
        (if (and (> 8e+01 (.roll _returnvalue)) (> (.roll _returnvalue) -8e+01))
          (Transformation|AddLocalRotation (Variables|Default|Getbird) (Math|Rotator|MakeRotator (Variables|Default|GetDecay) 0.0 0.0) false false))))))

(event Input|ActionEvents|InputActionJump
  (params (Key :type Key%20Structure :default "None"))
  (bind _bird (Variables|Default|Getbird))
  (bind _returnvalue (Transformation|GetWorldRotation _bird))
  ;[1 1 1] Impulse to fly
  (:Pressed
    (Variables|Default|SetEstaCaindo false)
    (Physics|AddImpulse (Variables|Collision|GetCapsuleComponent) (Math|Vector|MakeVector 0.0 0.0 (* (Variables|Default|GetImpluseMultiplier) (Variables|Default|GetImpulse%20Z))) "None" false)
    (if (and (> (.roll _returnvalue) 0.0) (> 85.0 (.roll _returnvalue)))
      (Transformation|AddLocalRotation (Variables|Default|Getbird) (Math|Rotator|MakeRotator (Variables|Default|GetSustain) 0.0 0.0) false false)))
  (:Released
    (Variables|Default|SetEstaCaindo true)))

(fn ConstructionScript)