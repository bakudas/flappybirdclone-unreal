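; Spawner actor that creates pairs of pipe obstacles with a score zone, in the style of Flappy Bird.
; A Delay on Tick acts as a repeating 1.2-second timer, each cycle nudging the actor by a random, cumulative Z offset.
; CreatePipes then spawns BP_Pipe at two spawn points, one rotated 180 degrees in yaw.
; A BP_ScoreZone follows at the root's Y and Z with a fixed world X.
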(event EventBeginPlay)

(event EventTick
  (params (DeltaSeconds :type Float%20%28single-precision%29))
  (bind _defaultsceneroot (Variables|Default|GetDefaultSceneRoot))
  (bind _returnvalue (Transformation|GetWorldLocation _defaultsceneroot))
  (Utilities|FlowControl|Delay 1.2)
  (Class|Actor|AddActorLocalTransform (Math|Transform|MakeTransform (Math|Vector|MakeVector 0.0 0.0 (Math|Random|RandomFloatinRange -5e+01 5e+01)) "0, 0, 0" "1,1,1") false false)
  (CallFunction|CreatePipes)
  (Game|SpawnActorfromClass "/Game/Blueprints/BP_ScoreZone.BP_ScoreZone_C" (Math|Transform|MakeTransform (Math|Vector|MakeVector 1e+01 (.y _returnvalue) (.z _returnvalue)) "0, 0, 0" "1,1,1") "Undefined" 0 0))

(fn ConstructionScript)

(fn CreatePipes
  (Game|SpawnActorfromClass "/Game/Blueprints/BP_Pipe.BP_Pipe_C" (Math|Transform|MakeTransform (Transformation|GetWorldLocation (Variables|Default|GetSpawnPoint1)) "180.000000, 0, 0" "1,1,1") "Undefined" 0 0)
  (Game|SpawnActorfromClass "/Game/Blueprints/BP_Pipe.BP_Pipe_C" (Math|Transform|MakeTransform (Transformation|GetWorldLocation (Variables|Default|GetSpawnPoint2)) "0, 0, 0" "1,1,1") "Undefined" 0 0))